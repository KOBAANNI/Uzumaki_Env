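; Sky_BP is a sky sphere actor that styles the environment's sky through material parameters on its SkySphere component.
; Its Construction Script pushes sky, horizon and sun colors plus sun size into those materials.
; The sun direction comes from the forward vector of a referenced SunDirection actor's rotation.
; The event graph holds only disabled stubs, so nothing updates in BeginPlay or Tick.
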(fn `UserConstructionScript`
  (bind _skysphere (`self.SkySphere`))
  (`MeshComponent.SetVectorParameterValueOnMaterials` _skysphere "SkyColor" (`KismetMathLibrary.Conv_LinearColorToVector` (`self.SkyColor`)))
  (`MeshComponent.SetVectorParameterValueOnMaterials` _skysphere "HorizonColor" (`KismetMathLibrary.Conv_LinearColorToVector` (`self.HorizonColor`)))
  (`MeshComponent.SetVectorParameterValueOnMaterials` _skysphere "SunDirection" (`KismetMathLibrary.Conv_RotatorToVector` (`self.K2_GetActorRotation` (`self.SunDirection`))))
  (`MeshComponent.SetVectorParameterValueOnMaterials` _skysphere "SunColor" (`KismetMathLibrary.Conv_LinearColorToVector` (`self.SunColor`)))
  (`MeshComponent.SetScalarParameterValueOnMaterials` (`self.SkySphere`) "SunSize" (`self.SunSize`)))