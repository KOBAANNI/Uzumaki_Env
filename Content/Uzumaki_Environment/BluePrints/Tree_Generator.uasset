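; Procedural tree actor that builds a trunk and optional branches from spline meshes along an editable spline in its Construction Script.
; It resizes TreeDataArray to match the spline points, giving each point bend, thickness and left/right leaf settings.
; Each segment gets a trunk mesh plus any flagged branch meshes on the same curve, with roll and scale taken from its endpoints.
; Collision, loop closing and point-number text labels are optional.
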(fn `BuildTreeElement`
  (params (LoopIndex :type Integer) (TreeElementMesh :type "StaticMesh Object Reference"))
  (locals (Local_CurrentLoopIndex :type Integer) (Local_NextLoopIndex :type Integer) (Local_TrackElementMesh :type "StaticMesh Object Reference") (Local_StartLocation :type "Vector Structure") (Local_StartTangent :type "Vector Structure") (Local_EndLocation :type "Vector Structure") (Local_EndTangent :type "Vector Structure") (Local_CurrentSplineMesh :type "SplineMeshComponent Object Reference") (Local_StartRoll :type "Float (double-precision)") (Local_StartScale :type "Vector2D Structure") (Local_EndRoll :type "Float (double-precision)") (Local_EndScale :type "Vector2D Structure"))
  (bind _local_currentsplinemesh (`local.Local_CurrentSplineMesh`))
  (bind _local_currentsplinemesh_2 (`local.Local_CurrentSplineMesh`))
  (bind (_location _tangent) (`SplineComponent.GetLocationAndTangentAtSplinePoint` (`self.Spline`) (`local.Local_NextLoopIndex`) "Local"))
  (bind (_location_2 _tangent_2) (`SplineComponent.GetLocationAndTangentAtSplinePoint` (`self.Spline`) (`local.Local_CurrentLoopIndex`) "Local"))
  (bind (_output_leftleaf _output_rightleaf _output_treebend _output_treethickness) (break `/Game/Uzumaki_Environment/BluePrints/Data/Tree_Data` (`|GetArrayItem` (`self.TreeDataArray`) (`local.Local_NextLoopIndex`))))
  (bind (_output_leftleaf_2 _output_rightleaf_2 _output_treebend_2 _output_treethickness_2) (break `/Game/Uzumaki_Environment/BluePrints/Data/Tree_Data` (`|GetArrayItem` (`self.TreeDataArray`) (`local.Local_CurrentLoopIndex`))))
  (bind _output_get (set `local.Local_CurrentLoopIndex` LoopIndex))
  (set `local.Local_NextLoopIndex` (mod (+ _output_get 1) (`self.Number of Spline Points`)))
  (set `local.Local_TrackElementMesh` TreeElementMesh)
  (`|ExecutionSequence`
    (:`then_0`
      (set `local.Local_StartLocation` _location_2)
      (set `local.Local_StartTangent` _tangent_2)
      (set `local.Local_EndLocation` _location)
      (set `local.Local_EndTangent` _tangent)
      (set `local.Local_StartRoll` _output_treebend_2)
      (set `local.Local_StartScale` (`KismetMathLibrary.MakeVector2D` _output_treethickness_2 _output_treethickness_2))
      (set `local.Local_EndRoll` _output_treebend)
      (set `local.Local_EndScale` (`KismetMathLibrary.MakeVector2D` _output_treethickness _output_treethickness)))
    (:`then_1`
      (bind _returnvalue (`AddComponent|NODE_AddSplineMeshComponent-0`))
      (bind _output_get_2 (set `local.Local_CurrentSplineMesh` _returnvalue))
      (`StaticMeshComponent.SetStaticMesh` _output_get_2 (`local.Local_TrackElementMesh`))
      (`SplineMeshComponent.SetForwardAxis` _returnvalue (`self.FowardAxis`) true)
      (`SceneComponent.K2_AttachToComponent` _returnvalue (`local.Local_CurrentSplineMesh`) "None" "KeepRelative" "KeepRelative" "KeepRelative" true)
      (`SplineMeshComponent.SetStartAndEnd` (`local.Local_CurrentSplineMesh`) (`local.Local_StartLocation`) (`local.Local_StartTangent`) (`local.Local_EndLocation`) (`local.Local_EndTangent`) true)
      (`SplineMeshComponent.SetStartRoll` _local_currentsplinemesh (`local.Local_StartRoll`) true)
      (`SplineMeshComponent.SetEndRoll` _local_currentsplinemesh (`local.Local_EndRoll`) true)
      (`SplineMeshComponent.SetStartScale` _local_currentsplinemesh_2 (`local.Local_StartScale`) true)
      (`SplineMeshComponent.SetEndScale` _local_currentsplinemesh_2 (`local.Local_EndScale`) true)
      (`PrimitiveComponent.SetCollisionEnabled` (`local.Local_CurrentSplineMesh`) (select `bool` (`self.Collisions`) :`false` "NoCollision" :`true` "QueryAndPhysics" :!type "ECollisionEnabled Enum")))))

(fn `UserConstructionScript`
  (bind _treedataarray (`self.TreeDataArray`))
  (bind (_output_leftleaf _output_rightleaf) (break `/Game/Uzumaki_Environment/BluePrints/Data/Tree_Data` (`|GetArrayItem` (`self.TreeDataArray`) (`self.Current Loop Index`))))
  (`|ExecutionSequence`
    (:`then_0`
      (set `self.Number of Spline Points` (`SplineComponent.GetNumberOfSplinePoints` (`self.Spline`))))
    (:`then_1`
      (`/Engine/EditorBlueprintResources/StandardMacros.CompareInt` (`KismetArrayLibrary.Array_Length` (`self.TreeDataArray`)) (`self.Number of Spline Points`) :!label _label
        (:`>`
          (`KismetArrayLibrary.Array_Remove` _treedataarray (`KismetArrayLibrary.Array_LastIndex` _treedataarray))
          (goto _label))
        (:`<`
          (`KismetArrayLibrary.Array_Add` (`self.TreeDataArray`) (`self.Tree Mesh Deaults`))
          (goto _label))))
    (:`then_2`
      (for _index (range (+ (- (`self.Number of Spline Points`) (`KismetMathLibrary.SelectInt` 1 2 (`self.Looping Track`))) 1))
        (set `self.Current Loop Index` _index)
        (set `self.Draw Left Branch` _output_leftleaf)
        (set `self.Draw Right Branch` _output_rightleaf)
        (`|ExecutionSequence`
          (:`then_0`
            (`self.BuildTreeElement` (`self.Current Loop Index`) (`self.Tree Mesh`)))
          (:`then_1`
            (if (`self.Draw Left Branch`)
              (`self.BuildTreeElement` (`self.Current Loop Index`) (`self.Left branch mesh`))))
          (:`then_2`
            (if (`self.Draw Right Branch`)
              (`self.BuildTreeElement` (`self.Current Loop Index`) (`self.Right branch mesh`)))))))
    (:`then_3`
      (if (`self.Draw Track Point Numbers`)
        (for _index_2 (range (`self.Number of Spline Points`))
          (bind _output_get (set `self.Current track type` (`KismetStringLibrary.Conv_IntToString` _index_2)))
          (bind (_location _tangent) (`SplineComponent.GetLocationAndTangentAtSplinePoint` (`self.Spline`) _index_2 "Local"))
          (bind _returnvalue (`AddComponent|NODE_AddTextRenderComponent-0` :`RelativeTransform` (`KismetMathLibrary.MakeTransform` (`KismetMathLibrary.MakeVector` (.x _location) (.y _location) (+ (.z _location) 50.0)) (`KismetMathLibrary.Conv_VectorToRotator` (* _tangent -1.0)))))
          (`TextRenderComponent.K2_SetText` _returnvalue (`KismetTextLibrary.Conv_StringToText` _output_get)))))))