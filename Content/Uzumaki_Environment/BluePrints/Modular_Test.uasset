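; Modular building test Blueprint that procedurally assembles a front wall from tiled static meshes.
; The Construction Script loops over floor and column counts, spacing pieces by tile size along X and Z, with MeshTop on the top floor and Wall below.
; A CreateMesh helper adds and assigns each Static Mesh Component.
; Only the front side is built, and the event graph has no active logic.
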(fn `Create Mesh`
  (params (Transform :type "Transform Structure") (Mesh :type "StaticMesh Object Reference"))
  (bind _returnvalue (`AddComponent|NODE_AddStaticMeshComponent-0` :`RelativeTransform` Transform))
  (`StaticMeshComponent.SetStaticMesh` _returnvalue Mesh)
  (`PrimitiveComponent.SetMaterial` _returnvalue 0 null)
  (`PrimitiveComponent.SetMaterial` _returnvalue 0 null))

(fn `UserConstructionScript`
  (bind _returnvalue (- (`self.Number of Floors`) 1))
  (`|ExecutionSequence`
    (:`then_0`
      ;[1 1 1] Front
      (for _index (range (+ _returnvalue 1))
        (for _index_2 (range (`self.Number of X`))
          (`|ExecutionSequence`
            (:`then_0`
              (if (== _index _returnvalue)
                (`self.Create Mesh` (`KismetMathLibrary.MakeTransform` (`KismetMathLibrary.MakeVector` (* _index_2 (`self.X tile`)) 0.0 (* _index (`self.Z Tile`)))) (`self.Mesh Top`))
                (else
                  (`self.Create Mesh` (`KismetMathLibrary.MakeTransform` (`KismetMathLibrary.MakeVector` (* _index_2 (`self.X tile`)) 0.0 (* _index (`self.Z Tile`)))) (`self.Wall`)))))))))))